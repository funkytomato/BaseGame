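; Base armed combat character that handles weapon selection, shooting, reloading, aiming and grenade-throw montages.
; Number keys or events toggle three socket-attached child-actor guns, while shoot calls EquippedGun and reload calls PrimaryGun.
; A separate four-slot inventory, seeded at BeginPlay alongside the HUD, cycles weapons by copying data table stats into current-weapon variables, with clients sending a server event for effects fields.
; SetWeaponEquipped is empty, so cycling leaves gun actors unchanged.
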(event `Svr_SetActiveWpmVars`
  (params (InventorySlot :type Integer))
  ;[1 1 1] Server Set Active Weapon Variables
  (`self.ServerSetActiveWpnVars` InventorySlot))

(event `self.ReceiveBeginPlay`
  ;[1 1 1] BeginPlay - Equip Weapon and get animation reference
  (`parent.ReceiveBeginPlay`)
  (`self.SelectPrimaryWeapon`)
  (bind _asarmed_combat_master_anim_bp (cast `/Game/MyContent/Blueprints/Characters/ArmedCombatMaster_AnimBP` (`SkeletalMeshComponent.GetAnimInstance` (`self.Mesh`))))
  (set `self.AnimInstanceRef` _asarmed_combat_master_anim_bp)
  (`self.HUDandWeaponInventory`))

(event `HUDandWeaponInventory`
  (bind _returnvalue (`|CreateWidget` "/Game/MyContent/UI/PlayerHUD.PlayerHUD_C" (`GameplayStatics.GetPlayerController` 0)))
  (`UserWidget.AddToViewport` _returnvalue 0)
  (`self.AddToWeaponInventory` "Rifle" 0 150 30)
  (`self.AddToWeaponInventory` "Shotgun" 1 36 6)
  (`self.AddToWeaponInventory` "Sidearm" 2 64 9)
  (`self.AddToWeaponInventory` "Assault" 3 210 25)
  (`self.SetActiveWpnVars` 0))

(event `SelectPrimaryWeapon`
  ;[1 1 1] Weapon Selection
  (set `self.CurrentlyEquipped` 0 :!label _label)
  (`self.EquipGun`))

(event `InputAction|Reload`
  (params (Key :type "Key Structure"))
  ;[1 1 1] Reload Weapon
  (:`Pressed`
    (bind _asgun_master_bp (cast `/Game/MyContent/Guns/GunMaster_BP` (`ChildActorComponent.ChildActor` (`self.PrimaryGun`))))
    (`/Game/MyContent/Guns/GunMaster_BP.Reload` _asgun_master_bp)))

(event `InputAction|PrimaryWeapon`
  (params (Key :type "Key Structure"))
  ;[1 1 1] Weapon Selection
  (:`Pressed`
    (goto _label)))

(event `SelectSecondaryWeapon`
  ;[1 1 1] Weapon Selection
  (set `self.CurrentlyEquipped` 1 :!label _label_2)
  (`self.EquipGun`))

(event `InputAction|SecondaryWeapon`
  (params (Key :type "Key Structure"))
  ;[1 1 1] Weapon Selection
  (:`Pressed`
    (goto _label_2)))

(event `InputAction|SideArm`
  (params (Key :type "Key Structure"))
  ;[1 1 1] Weapon Selection
  (:`Pressed`
    (set `self.CurrentlyEquipped` 2 :!label _label_3)
    (`self.EquipGun`)))

(event `SelectSideArm`
  (goto _label_3))

(event `StartShooting`
  ;[1 1 1] Shooting Sequence
  (set `self.IsShooting` true :!label _label_4)
  (`/Game/MyContent/Guns/GunMaster_BP.StartShooting` (`self.EquippedGun`))
  (`|PlayMontage` (`self.Mesh`)
    (:`then`
      (`KismetSystemLibrary.PrintString` "Shooting"))))

(event `InputAction|Shoot`
  (params (Key :type "Key Structure"))
  ;[1 1 1] Shooting Sequence
  (:`Pressed`
    (goto _label_4))
  (:`Released`
    (set `self.IsShooting` false :!label _label_5)
    (`/Game/MyContent/Guns/GunMaster_BP.StopShooting` (`self.EquippedGun`))))

(event `InputAction|CycleWeaponUp`
  (params (Key :type "Key Structure"))
  ;[1 1 1] Cycle Weapons Up
  (:`Pressed`
    (set `self.SwitchToSlotNbr` (`self.ActiveWpnSlot`))
    ;;[1 1 1] If slot nbr > array size
    (if (> (+ (`self.SwitchToSlotNbr`) 1) (- (`KismetArrayLibrary.Array_Length` (`self.WeapInvNames`)) 1)) :!label _label_6
      ;;[1 1 1] Go to slot 0
      (set `self.SwitchToSlotNbr` 0)
      (else
        ;;[1 1 1] Go to next slot
        (set `self.SwitchToSlotNbr` (+ (`self.SwitchToSlotNbr`) 1))))
    ;;[1 1 1] If all weapons checjked
    (if (not (== (`self.SwitchToSlotNbr`) (`self.ActiveWpnSlot`)))
      (bind _canswitchweapon (`self.CanSwitchWeapon` (`self.SwitchToSlotNbr`)))
      (if _canswitchweapon
        (bind _output_get (set `self.ActiveWpnSlot` (`self.SwitchToSlotNbr`)))
        (`self.SetActiveWpnVars` _output_get)
        (`self.SetWeaponEquipped`)
        (else
          (goto _label_6))))))

(event `StopShooting`
  ;[1 1 1] Shooting Sequence
  (goto _label_5))

(event `InputAction|Aim`
  (params (Key :type "Key Structure"))
  (bind _returnvalue (`SkeletalMeshComponent.GetAnimInstance` (`self.Mesh`)))
  ;[1 1 1] Aim
  (:`Pressed`
    (set `self.IsAiming?` true)
    (bind _asarmed_combat_master_anim_bp (cast `/Game/MyContent/Blueprints/Characters/ArmedCombatMaster_AnimBP` _returnvalue))
    (set `/Game/MyContent/Blueprints/Characters/ArmedCombatMaster_AnimBP.IsAiming` true _asarmed_combat_master_anim_bp)
    (set `/Game/MyContent/Blueprints/Characters/MasterCharacter_AnimBP.IsADS?` true _asarmed_combat_master_anim_bp))
  (:`Released`
    (set `self.IsAiming?` false)
    (bind _asarmed_combat_master_anim_bp_2 (cast `/Game/MyContent/Blueprints/Characters/ArmedCombatMaster_AnimBP` _returnvalue))
    (set `/Game/MyContent/Blueprints/Characters/ArmedCombatMaster_AnimBP.IsAiming` false _asarmed_combat_master_anim_bp_2)
    (set `/Game/MyContent/Blueprints/Characters/MasterCharacter_AnimBP.IsADS?` false _asarmed_combat_master_anim_bp_2)))

(event `Threatened`
  ;[1 1 1] Threatened
  (set `self.IsInDanger?` true)
  (`KismetSystemLibrary.PrintString` "Threatened!!!"))

(event `InputAction|CycleWeaponDown`
  (params (Key :type "Key Structure"))
  ;[1 1 1] Cycle Weapons Down
  (:`Pressed`
    (set `self.SwitchToSlotNbr` (`self.ActiveWpnSlot`))
    ;;[1 1 1] If slot nbr < 0
    (if (< (- (`self.SwitchToSlotNbr`) 1) 0) :!label _label_7
      ;;[1 1 1] Go to highest slot
      (set `self.SwitchToSlotNbr` (- (`KismetArrayLibrary.Array_Length` (`self.WeapInvNames`)) 1))
      (else
        ;;[1 1 1] Go to previous slot
        (set `self.SwitchToSlotNbr` (- (`self.SwitchToSlotNbr`) 1))))
    ;;[1 1 1] If all weapons checjked
    (if (not (== (`self.SwitchToSlotNbr`) (`self.ActiveWpnSlot`)))
      (bind _canswitchweapon (`self.CanSwitchWeapon` (`self.SwitchToSlotNbr`)))
      (if _canswitchweapon
        (bind _output_get (set `self.ActiveWpnSlot` (`self.SwitchToSlotNbr`)))
        (`self.SetActiveWpnVars` _output_get)
        (`self.SetWeaponEquipped`)
        (else
          (goto _label_7))))))

(event `ThrowGrenade`
  (bind _charactermovement (`self.CharacterMovement`))
  (bind _grenadethrowmontages (`self.GrenadeThrowMontages`))
  (if (`NavMovementComponent.IsFalling` (`self.CharacterMovement`))
    _
    (elif (not (`self.IsThrowingGrenade?`))
      (set `self.IsAttacking?` true)
      (set `self.IsThrowingGrenade?` true)
      (`CharacterMovementComponent.DisableMovement` _charactermovement)
      (bind _returnvalue (`self.PlayAnimMontage` (`|GetArrayItem` _grenadethrowmontages (`KismetMathLibrary.RandomIntegerInRange` 0 (`KismetArrayLibrary.Array_Length` _grenadethrowmontages)))))
      (`KismetSystemLibrary.Delay` _returnvalue)
      (`CharacterMovementComponent.SetMovementMode` _charactermovement "MOVE_Walking" 0)
      (set `self.IsThrowingGrenade?` false)
      (set `self.IsAttacking?` false))))

(event `CancelThrow`
  (bind _cancelgrenadethrowmontages (`self.CancelGrenadeThrowMontages`))
  (bind _charactermovement (`self.CharacterMovement`))
  (if (`NavMovementComponent.IsFalling` (`self.CharacterMovement`))
    _
    (elif (not (`self.IsCancelGrenadeThrow?`))
      (set `self.IsAttacking?` true)
      (set `self.IsCancelGrenadeThrow?` true)
      (`CharacterMovementComponent.DisableMovement` _charactermovement)
      (bind _returnvalue (`self.PlayAnimMontage` (`|GetArrayItem` _cancelgrenadethrowmontages (`KismetMathLibrary.RandomIntegerInRange` 0 (`KismetArrayLibrary.Array_Length` _cancelgrenadethrowmontages)))))
      (`KismetSystemLibrary.Delay` _returnvalue)
      (`CharacterMovementComponent.SetMovementMode` _charactermovement "MOVE_Walking" 0)
      (set `self.IsCancelGrenadeThrow?` false)
      (set `self.IsAttacking?` false))))

(fn `AddToWeaponInventory`
  (params (WeapRowName :type Name) (InventorySlot :type Integer) (StartAmmoStock :type Integer) (StartAmmoClip :type Integer))
  (`KismetArrayLibrary.Array_Set` (`self.WeapInvNames`) InventorySlot WeapRowName true)
  (`KismetArrayLibrary.Array_Set` (`self.CW_AmmoStock`) InventorySlot StartAmmoStock true)
  (`KismetArrayLibrary.Array_Set` (`self.CW_AmmoClip`) InventorySlot StartAmmoClip true))

(fn `CanSwitchWeapon`
  (params (NewWpnSlot :type Integer))
  (returns (CanSwitchWeapon :type Boolean))
  (if (> (`|GetArrayItem` (`self.CW_AmmoStock`) NewWpnSlot) 0)
    _
    (elif (> NewWpnSlot 0)
      _
      (else
        (return false))))
  (return true))

(fn `EquipGun`
  (bind _array (`|MakeArray` (`self.PrimaryGun`) (`self.SecondaryGun`) (`self.SideArmGun`)))
  (bind _output (`|GetArrayItem` _array (`self.CurrentlyEquipped`)))
  (for _array_element _array
    (`SceneComponent.SetVisibility` _array_element false false))
  (`SceneComponent.SetVisibility` _output true false)
  (`SceneComponent.K2_AttachToComponent` _output (`self.Mesh`) "WeaponSocket" "SnapToTarget" "SnapToTarget" "SnapToTarget" true))

(fn `ServerSetActiveWpnVars`
  (params (InventorySlot :type Integer))
  (bind _returnvalue (`|GetDataTableRow` "/Game/MyContent/Blueprints/Weapons/Welded/WeaponInfoTable.WeaponInfoTable" (`|GetArrayItem` (`self.WeapInvNames`) InventorySlot))
    (:`then`
      (bind (_displayname _weapontype _firetype _shotcount _maxammostock _maxammoclip _firedelay _burstdelay _reloadtime _spread _rechamber _rechambertime _maxtotalrange _muzzlesocket _firesound _muzzleflash _impactfx _zoomfov _maxdamage _mindamage _maxdamagerange _mindamagerange _fireanim) (break `/Game/MyContent/Blueprints/Weapons/Welded/WeaponInfoStruct` _returnvalue))
      (set `self.CW_Muzzle` _muzzlesocket)
      (set `self.CW_FireSound` _firesound)
      (set `self.CW_MuzzleFlash` _muzzleflash)
      (set `self.CW_ImpactFX` _impactfx)
      (set `self.CW_FireAnim` _fireanim))))

(fn `SetActiveWpnVars`
  (params (InventroySlot :type Integer))
  (bind _returnvalue (`|GetDataTableRow` "/Game/MyContent/Blueprints/Weapons/Welded/WeaponInfoTable.WeaponInfoTable" (`|GetArrayItem` (`self.WeapInvNames`) InventroySlot))
    (:`then`
      (`/Engine/EditorBlueprintResources/ActorMacros.Switch Has Authority`
        (:`Authority`
          _)
        (:`Remote`
          (`self.Svr_SetActiveWpmVars` InventroySlot)))
      (bind (_displayname _weapontype _firetype _shotcount _maxammostock _maxammoclip _firedelay _burstdelay _reloadtime _spread _rechamber _rechambertime _maxtotalrange _muzzlesocket _firesound _muzzleflash _impactfx _zoomfov _maxdamage _mindamage _maxdamagerange _mindamagerange _fireanim) (break `/Game/MyContent/Blueprints/Weapons/Welded/WeaponInfoStruct` _returnvalue))
      (set `self.CW_DisplayName` _displayname)
      (set `self.CW_WeaponType` _weapontype)
      (set `self.CW_FireType` _firetype)
      (set `self.CW_ShotCount` _shotcount)
      (set `self.CW_MaxAmmoStock` _maxammostock)
      (set `self.CW_MaxAmmoClip` _maxammoclip)
      (set `self.CW_FireDelay` _firedelay)
      (set `self.CW_BurstDelay` _burstdelay)
      (set `self.CW_ReloadTime` _reloadtime)
      (set `self.CW_Spread` _spread)
      (set `self.CW_Rechamber` _rechamber)
      (set `self.CW_RechamberTime` _rechambertime)
      (set `self.CW_MaxTotalRange` _maxtotalrange)
      (set `self.CW_Muzzle` _muzzlesocket)
      (set `self.CW_FireSound` _firesound)
      (set `self.CW_MuzzleFlash` _muzzleflash)
      (set `self.CW_ImpactFX` _impactfx)
      (set `self.CW_ZoomFOV` _zoomfov)
      (set `self.CW_MaxDamage` _maxdamage)
      (set `self.CW_MinDamage` _mindamage)
      (set `self.CW_MaxDamageRange` _maxdamagerange)
      (set `self.CW_MinDamageRange` _mindamagerange)
      (set `self.CW_FireAnim` _fireanim))))

(fn `SetWeaponEquipped`)

(fn `SpawnProjectile`
  (returns (Success :type Boolean))
  (bind _returnvalue (`|SpawnActorFromClass` "/Game/FirstPersonBP/Blueprints/FirstPersonProjectile.FirstPersonProjectile_C" (`SceneComponent.GetSocketTransform` (`self.Mesh`) "WeaponSocket" "RTS_World") "AlwaysSpawn" "OverrideRootScale" self null))
  (return (`KismetSystemLibrary.IsValid` _returnvalue)))

(fn `UserConstructionScript`
  (`parent.UserConstructionScript`)
  (bind _asgun_master_bp (cast `/Game/MyContent/Guns/GunMaster_BP` (`ChildActorComponent.ChildActor` (`self.PrimaryGun`))))
  (set `self.EquippedGun` _asgun_master_bp)
  (`SceneComponent.K2_AttachToComponent` (`self.PrimaryGun`) (`self.Mesh`) "WeaponSocket" "SnapToTarget" "SnapToTarget" "SnapToTarget" true))