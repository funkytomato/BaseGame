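; Base melee combat character that carries a weapon and deals damage to NPCs.
; Construction snaps the child-actor weapon to the mesh's SwordSocket, and BeginPlay caches the anim instance and weapon actor.
; Attack input only toggles an IsAttacking flag; montage playback exists but is unwired.
; MeleeCollision overlaps apply point damage to NPC-tagged actors other than itself, without checking the attack flag.
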(event `self.ReceiveBeginPlay`
  (`parent.ReceiveBeginPlay`)
  (bind _asmelee_combat_master_anim_bp (cast `/Game/MyContent/Blueprints/Characters/MeleeCombatMaster_AnimBP` (`SkeletalMeshComponent.GetAnimInstance` (`self.Mesh`))))
  (set `self.AnimInstance` _asmelee_combat_master_anim_bp)
  (bind _asmelee_master_bp (cast `/Game/MyContent/Melee/MeleeMaster_BP` (`ChildActorComponent.ChildActor` (`self.WeaponComponent`))))
  (set `self.CurrentMelee` _asmelee_master_bp))

(event `self.ReceiveActorBeginOverlap`
  (params (OtherActor :type "Actor Object Reference"))
  (`parent.ReceiveActorBeginOverlap` OtherActor))

(event `InputAction|Attack`
  (params (Key :type "Key Structure"))
  (:`Pressed`
    (set `self.IsAttacking?` true))
  (:`Released`
    (set `self.IsAttacking?` false)))

(event `self.MeleeCollision.OnComponentBeginOverlap`
  (params (OverlappedComponent :type "PrimitiveComponent Object Reference") (OtherActor :type "Actor Object Reference") (OtherComp :type "PrimitiveComponent Object Reference") (OtherBodyIndex :type Integer) (bFromSweep :type Boolean) (SweepResult :type "HitResult Structure (by ref)"))
  (if (`self.ActorHasTag` OtherActor "NPC")
    (if (!= OtherActor self)
      (`GameplayStatics.ApplyPointDamage` OtherActor 1.0 (`.ImpactNormal` (`GameplayStatics.BreakHitResult` SweepResult)) SweepResult null self "/Script/Engine.DamageType"))))

(fn `UserConstructionScript`
  (`parent.UserConstructionScript`)
  (`SceneComponent.K2_AttachToComponent` (`self.WeaponComponent`) (`self.Mesh`) "SwordSocket" "SnapToTarget" "SnapToTarget" "SnapToTarget" true))